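; SwitchBP is a switch that changes how many ships go after, presumably in pursuit, through the NumShipsGoAfter value on EscapeInSpaceGameInstance.
; An overlap on its Trigger component by an actor tagged Player calls Toggle.
; The OnEnable event raises the count and OnDisable lowers it to one, also printing a debug message.
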(event `self.OnEnable`
  (bind _asescape_in_space_game_instance (cast `/Game/Blueprints/EscapeInSpaceGameInstance` (`GameplayStatics.GetGameInstance`)))
  (set `/Game/Blueprints/EscapeInSpaceGameInstance.NumShipsGoAfter` 5 _asescape_in_space_game_instance))

(event `self.OnDisable`
  (`KismetSystemLibrary.PrintString` "Anssi is disabled.")
  (bind _asescape_in_space_game_instance (cast `/Game/Blueprints/EscapeInSpaceGameInstance` (`GameplayStatics.GetGameInstance`)))
  (set `/Game/Blueprints/EscapeInSpaceGameInstance.NumShipsGoAfter` 1 _asescape_in_space_game_instance))

(event `self.Trigger.OnComponentBeginOverlap`
  (params (OverlappedComponent :type "PrimitiveComponent Object Reference") (OtherActor :type "Actor Object Reference") (OtherComp :type "PrimitiveComponent Object Reference") (OtherBodyIndex :type Integer) (bFromSweep :type Boolean) (SweepResult :type "HitResult Structure (by ref)"))
  (if (`self.ActorHasTag` OtherActor "Player")
    (`self.Toggle`)))

(fn `UserConstructionScript`)