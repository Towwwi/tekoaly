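; Robot Blueprint that plays a name-writing material animation ("Seppo") when an actor tagged Player hits its capsule.
; The construction script puts a dynamic instance of SeppoMaterial on the static mesh.
; A hit resets AnimationPosition and starts a looping timer, unless one is already running.
; Each timer tick steps the material's scalar parameter, prints debug text, and clears the timer past a threshold.
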(event `self.CapsuleComponent.OnComponentHit`
  (params (HitComponent :type "PrimitiveComponent Object Reference") (OtherActor :type "Actor Object Reference") (OtherComp :type "PrimitiveComponent Object Reference") (NormalImpulse :type "Vector Structure") (Hit :type "HitResult Structure (by ref)"))
  (if (`self.ActorHasTag` OtherActor "Player")
    (`self.FixNameToSeppo`)))

(fn `FixNameToSeppo`
  (if (not (`KismetSystemLibrary.K2_IsValidTimerHandle` (`self.WritingTimer`)))
    (set `self.AnimationPosition` 0.0)
    (bind _returnvalue (`KismetSystemLibrary.K2_SetTimer` null "UpdateNameWriting" 0.1 true))
    (set `self.WritingTimer` _returnvalue)))

(fn `UpdateNameWriting`
  (bind _returnvalue (+ (`self.AnimationPosition`) 0.1))
  (`KismetSystemLibrary.PrintString` (`KismetStringLibrary.Concat_StrStr` "setting material to" (`KismetStringLibrary.Conv_DoubleToString` _returnvalue)))
  (set `self.AnimationPosition` _returnvalue)
  (bind _asmaterial_instance_dynamic (cast `MaterialInstanceDynamic` (`PrimitiveComponent.GetMaterial` (`self.StaticMesh`) 0)))
  (`MaterialInstanceDynamic.SetScalarParameterValue` _asmaterial_instance_dynamic "AnimationPosition" _returnvalue)
  (if (> _returnvalue 0.8)
    (`KismetSystemLibrary.K2_ClearAndInvalidateTimerHandle` (`self.WritingTimer`))))

(fn `UserConstructionScript`
  (bind _returnvalue (`KismetMaterialLibrary.CreateDynamicMaterialInstance` "/Game/Robot/SeppoMaterial.SeppoMaterial"))
  (`PrimitiveComponent.SetMaterial` (`self.StaticMesh`) 0 _returnvalue))