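; Ship engine component Blueprint that decides whether a boost can fire based on available charge.
; TryBoost checks TargetSource for enough charge to cover BurstConsumptionRate, then calls ConsumeBurst and returns its result as CanBoost.
; When charge is short, it returns false along with the missing energy amount.
; The event graph holds only disabled default events, so the component runs no tick logic of its own here.
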(fn `TryBoost`
  (returns (CanBoost :type Boolean) (`Missing Energy` :type "Float (double-precision)"))
  (bind _returnvalue (`EnergySource.HasCharge` (`self.TargetSource`) (`self.BurstConsumptionRate`)))
  (if _returnvalue
    (bind _returnvalue_2 (`self.ConsumeBurst`))
    (return _returnvalue_2 0.0)
    (else
      (return false (- (`self.BurstConsumptionRate`) (`EnergySource.GetCharge` (`self.TargetSource`)))))))